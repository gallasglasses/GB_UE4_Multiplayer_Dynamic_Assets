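; Multiplayer player character with axis-driven movement, jumping, projectile firing and health.
; Left click routes through server-named events to spawn BP_Projectile at the Direction component, with a timer resetting the fire-rate gate.
; HealthComponent takes damage and drives health text, the health bar widget and death, which blocks firing, disables movement and sets a short life span.
; A separate event possesses a spawned spectator pawn, but nothing here calls it; OnRep_Health is empty.
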(event Custom|Server_Fire
  ;[1 0.3114 0] Fire
  (if (Variables|Fire|GetbReadyToFire)
    (Variables|Fire|SetbReadyToFire false)
    (CallFunction|ServerShot)
    (Utilities|Time|SetTimerbyFunctionName self "Client_Reload" (Variables|Fire|GetFireRifleRate))
    (else
      (Development|PrintString "Not ready"))))

(event Custom|Server_SetHealthText
  (params (NewHealth :type Float%20%28single-precision%29))
  ;[0.09208 1 0] SetHealthBar
  (Rendering|Components|TextRender|SetText (Variables|Default|GetHealthTextRender) (Utilities|Text|ToText(Float) NewHealth "HalfToEven")))

(event Custom|OnDeath
  ;[0 0 0] OnDeath
  (Variables|Default|SetbIsDead true)
  (Development|PrintString "Is Dead")
  (Pawn|Components|CharacterMovement|DisableMovement (Variables|Character|GetCharacterMovement))
  (Actor|SetLifeSpan 5.0))

(event Custom|MakeDamage
  (params (Damage :type Float%20%28single-precision%29))
  ;[1 0 0] MakeDamage
  (Default|ServerTakeDamage (Variables|Default|GetHealthComponent) Damage))

(event Custom|OnHealthChanged
  (params (NewHealth :type Float%20%28single-precision%29))
  ;[0.5491 1 0.4844] OnHealthChanged
  (bind _output_get (Variables|Default|SetHealth NewHealth))
  (CallFunction|ServerSetHealthText _output_get)
  (CallFunction|ServerSetHealthBar))

(event Custom|Server_SetHealthBar
  ;[0.09208 1 0] SetHealthBar
  (bind _aswbp_health_bar (Utilities|Casting|CastToWBP_HealthBar (UserInterface|GetUserWidgetObject (Variables|Default|GetHealthBar))))
  (bind _healthpercent (Default|GetHealthPercent (Variables|Default|GetHealthComponent)))
  (Default|SetHealthPercent _aswbp_health_bar _healthpercent))

(event Custom|SetSpectatorAfterPawnDeath
  ;[1 0.03433 0.4129] Set Spectator after pawn death
  (bind _returnvalue (Game|SpawnActorfromClass "/Game/MMP_Content/Spectator/BP_SpectatorPawn.BP_SpectatorPawn_C" (Transformation|GetActorTransform) "Undefined" 0 0))
  (Pawn|Possess (Game|GetPlayerController 0) _returnvalue)
  (Variables|/Game/MMP_Content/Spectator/BP_SpectatorPawn.BP_SpectatorPawn_C|SetOG%20Player _returnvalue self))

(event Custom|Client_Reload
  ;[1 0.3114 0] Fire
  (Variables|Fire|SetbReadyToFire true)
  (Development|PrintString "Ready"))

(event Custom|Server_Shot
  (bind _self self)
  ;[1 0.3114 0] Fire
  (Game|SpawnActorfromClass "/Game/MMP_Content/Weapon/BP_Projectile.BP_Projectile_C" (Transformation|GetWorldTransform (Variables|Default|GetDirection)) "AlwaysSpawn" _self _self))

(event EventBeginPlay
  (bind _health (Default|GetHealth (Variables|Default|GetHealthComponent)))
  (CallFunction|OnHealthChanged _health)
  (EventDispatchers|BindEventtoOnDeath (Variables|Default|GetHealthComponent) (delegate Custom|OnDeath))
  (EventDispatchers|BindEventtoOnHealthChanged (Variables|Default|GetHealthComponent) (delegate Custom|OnHealthChanged)))

(event Collision|EventActorBeginOverlap
  (params (OtherActor :type Actor%20Object%20Reference)))

(event EventTick
  (params (DeltaSeconds :type Float%20%28single-precision%29)))

(event Input|ActionEvents|InputActionJump
  (params (Key :type Key%20Structure :default "None"))
  ;[0.006566 0.3073 0] Movement
  (:Pressed
    (Character|Jump))
  (:Released
    (Character|StopJumping)))

(event Input|AxisEvents|InputAxisTurn
  (params (AxisValue :type Float%20%28single-precision%29))
  ;[0.006566 0.3073 0] Movement
  (Pawn|Input|AddControllerYawInput AxisValue))

(event Input|AxisEvents|InputAxisLookUp
  (params (AxisValue :type Float%20%28single-precision%29))
  ;[0.006566 0.3073 0] Movement
  (Pawn|Input|AddControllerPitchInput AxisValue))

(event Input|AxisEvents|InputAxisMoveForward
  (params (AxisValue :type Float%20%28single-precision%29))
  ;[0.006566 0.3073 0] Movement
  (Pawn|Input|AddMovementInput (Math|Vector|GetForwardVector (Math|Rotator|MakeRotator 0.0 0.0 (.Yaw (Math|Rotator|BreakRotator (Pawn|GetControlRotation :!class /Script/Engine.Pawn))))) AxisValue false))

(event Input|AxisEvents|InputAxisMoveRight
  (params (AxisValue :type Float%20%28single-precision%29))
  ;[0.006566 0.3073 0] Movement
  (Pawn|Input|AddMovementInput (Math|Vector|GetRightVector (Math|Rotator|MakeRotator 0.0 0.0 (.Yaw (Math|Rotator|BreakRotator (Pawn|GetControlRotation :!class /Script/Engine.Pawn))))) AxisValue false))

(event Input|MouseEvents|LeftMouseButton
  (params (Key :type Key%20Structure :default "None"))
  ;[1 0.3114 0] Fire
  (:Pressed
    (if (not (Variables|Default|GetbIsDead))
      (CallFunction|ServerFire))))

(fn ConstructionScript)

(fn OnRepHealth)