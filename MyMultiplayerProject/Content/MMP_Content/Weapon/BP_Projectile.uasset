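; BP_Projectile is a multiplayer projectile that damages players and explodes on impact.
; The server moves it forward each tick by setting its location without sweep, and handles sphere overlaps.
; Hits ignore the owner and other projectiles, damage any BP_MultiplayerPlayer, multicast an explosion effect, then destroy the actor.
; A lifetime timer started on BeginPlay also destroys it through a server event.
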(event OnComponentBeginOverlap(SphereCollision)
  (params (OverlappedComponent :type Primitive%20Component%20Object%20Reference) (OtherActor :type Actor%20Object%20Reference) (OtherComp :type Primitive%20Component%20Object%20Reference) (OtherBodyIndex :type Integer) (bFromSweep :type Boolean) (SweepResult :type Hit%20Result%20Structure%20%28by%20ref%29))
  ;[1 0.3116 0.01834] Begin Overlap / Hit
  (if (Networking|IsServer)
    (CallFunction|ServeronProjectileHit OtherActor (Transformation|GetActorLocation))))

(event Custom|LifeEnded
  ;[0 0 0] Life Time
  (CallFunction|ServerLifeEnded))

(event Custom|Server_LifeEnded
  ;[0 0 0] Life Time
  (Actor|DestroyActor))

(event Custom|Server_Move
  (params (DeltaTime :type Float%20%28single-precision%29))
  ;[0.006566 0.3073 0] Movement
  (Transformation|SetActorLocation (+ (* (Transformation|GetActorForwardVector) (* DeltaTime (Variables|Float|GetSpeed))) (Transformation|GetActorLocation)) false false))

(event Custom|SpawnHitEffect
  (params (HitLocation :type Vector))
  ;[1 0.3116 0.01834] Begin Overlap / Hit
  (Effects|SpawnEmitteratLocation "/Game/StarterContent/Particles/P_Explosion.P_Explosion" HitLocation))

(event Custom|Multicast_HitEffect
  (params (HitLocation :type Vector))
  ;[1 0.3116 0.01834] Begin Overlap / Hit
  (CallFunction|SpawnHitEffect HitLocation))

(event Custom|Server_OnProjectileHit
  (params (OtherActor :type Actor%20Object%20Reference) (Location :type Vector))
  ;[1 0.3116 0.01834] Begin Overlap / Hit
  (if (!= OtherActor (Components|GetOwner))
    (bind _asbp_multiplayer_player (Utilities|Casting|CastToBP_MultiplayerPlayer OtherActor)
      (:then
        (Default|MakeDamage _asbp_multiplayer_player (Variables|Float|GetDamage)))
      (:CastFailed
        (Utilities|Casting|CastToBP_Projectile OtherActor
          (:CastFailed
            _))))
    (CallFunction|MulticastHitEffect Location)
    (CallFunction|ServerLifeEnded)))

(event EventBeginPlay
  ;[0 0 0] Life Time
  (Utilities|Time|SetTimerbyEvent (delegate Custom|LifeEnded) (Variables|Float|GetLifeTime)))

(event Collision|EventActorBeginOverlap
  (params (OtherActor :type Actor%20Object%20Reference)))

(event EventTick
  (params (DeltaSeconds :type Float%20%28single-precision%29))
  ;[0.006566 0.3073 0] Movement
  (if (Networking|IsServer)
    (CallFunction|ServerMove DeltaSeconds)))

(fn ConstructionScript)