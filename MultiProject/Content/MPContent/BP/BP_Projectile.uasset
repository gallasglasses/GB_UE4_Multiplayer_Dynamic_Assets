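; Multiplayer projectile actor that flies forward, damages characters on contact and expires after a set lifetime.
; The server moves it along its forward vector each tick without sweeping and handles shell overlaps, ignoring its owner and other projectiles.
; Any other hit multicasts a small explosion effect and destroys the projectile through the same server event the lifetime timer calls, with characters also taking damage.
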(event OnComponentBeginOverlap(Shell)
  (params (OverlappedComponent :type Primitive%20Component%20Object%20Reference) (OtherActor :type Actor%20Object%20Reference) (OtherComp :type Primitive%20Component%20Object%20Reference) (OtherBodyIndex :type Integer) (bFromSweep :type Boolean) (SweepResult :type Hit%20Result%20Structure%20%28by%20ref%29))
  ;[0.1825 0 0.4635] On Overlap and Check this
  (if (Networking|IsServer)
    (CallFunction|ServerCheckCollisionOverlap OtherActor (Transformation|GetActorLocation) SweepResult)))

(event Custom|LifeEnded
  ;[0 0 0] Life Ended
  (CallFunction|ServerLifeEnded))

(event Custom|Server_LifeEnded
  ;[0 0 0] Life Ended
  (Actor|DestroyActor))

(event Custom|Server_Move
  (params (DeltaTime :type Float%20%28single-precision%29))
  ;[0.4552 0.4552 0.4552] Movement
  (Transformation|SetActorLocation (+ (Transformation|GetActorLocation) (* (Transformation|GetActorForwardVector) (* DeltaTime (Variables|Default|GetSpeed)))) false false))

(event Custom|Server_CheckCollisionOverlap
  (params (OtherActor :type Actor%20Object%20Reference) (Location :type Vector) (HitResult :type Hit%20Result%20Structure))
  ;[0.1825 0 0.4635] On Overlap and Check this
  (if (!= OtherActor (Components|GetOwner))
    (bind _asbp_multiplayer_chararcter (Utilities|Casting|CastToBP_MultiplayerChararcter OtherActor)
      (:then
        (Default|MakeDamage _asbp_multiplayer_chararcter HitResult (Variables|Default|GetDamage)))
      (:CastFailed
        (Utilities|Casting|CastToBP_Projectile OtherActor
          (:CastFailed
            _))))
    (CallFunction|MulticastHitEffect Location)
    (CallFunction|ServerLifeEnded)))

(event Custom|SpawnHitEffects
  (params (HitLocation :type Vector))
  ;[1 0.3809 0.007211] Hit Effect
  (Effects|SpawnEmitteratLocation "/Game/StarterContent/Particles/P_Explosion.P_Explosion" HitLocation "0, 0, 0" "0.500000,0.500000,0.500000"))

(event Custom|Multicast_HitEffect
  (params (HitLocation :type Vector))
  ;[1 0.3809 0.007211] Hit Effect
  (CallFunction|SpawnHitEffects HitLocation))

(event EventBeginPlay
  (Utilities|Time|SetTimerbyEvent (delegate Custom|LifeEnded) (Variables|Default|GetTTL)))

(event Collision|EventActorBeginOverlap
  (params (OtherActor :type Actor%20Object%20Reference)))

(event EventTick
  (params (DeltaSeconds :type Float%20%28single-precision%29))
  (if (Networking|IsServer)
    (CallFunction|ServerMove DeltaSeconds)))

(fn ConstructionScript)