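; Actor component that tracks its owner's health, reduces it on any damage, and supports optional auto-healing.
; All changes pass through SetHealth, which clamps to MaxHealth and fires OnHealthChanged with the delta.
; Damage stops any running heal timer, then either fires OnDeath or, with AutoHeal on, starts a delayed looping HealUpdate timer until full.
; Health has a RepNotify function, currently empty, and the graphs contain no authority checks.
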(event Custom|OnTakeAnyDamage
  (params (DamagedActor :type Actor%20Object%20Reference) (Damage :type Float%20%28single-precision%29) (DamageType :type Damage%20Type%20Object%20Reference) (InstigatedBy :type Controller%20Object%20Reference) (DamageCauser :type Actor%20Object%20Reference))
  ;[1 1 1 0.2] Check: Can we take damage?
  (bind _bisdead (CallFunction|IsDead))
  (if (not (or _bisdead (<= Damage 0.0)))
    (CallFunction|SetHealth (- (Variables|Default|GetHealth) Damage))
    ;[1 1 1 0.2] Turn off Heal-timer because of damage
    (Utilities|Time|ClearandInvalidateTimerbyHandle (Variables|Heal|GetHealTimer))
    ;[1 1 1 0.2] Check: Is player dead now or not?
    (bind _bisdead_2 (CallFunction|IsDead))
    (if _bisdead_2
      ;[1 1 1 0.2] yep
      (Default|CallOnDeath)
      (else
        ;[1 1 1 0.2] Congrats, u r alive! If autoheal turn on, so it work. else you will say "i need healing" all the time
        (if (Variables|Heal|GetbAutoHeal)
          (bind _returnvalue (Utilities|Time|SetTimerbyFunctionName self "HealUpdate" (Variables|Heal|GetHealUpdateTime) true (Variables|Heal|GetHealDelay)))
          (Variables|Heal|SetHealTimer _returnvalue))))))

(event EventBeginPlay
  (bind _returnvalue (Components|GetOwner))
  (bind _maxhealth (Variables|Default|GetMaxHealth))
  (if (> _maxhealth 0.0)
    (CallFunction|SetHealth _maxhealth)
    (Utilities|IsValid _returnvalue
      (:Is%20Valid
        (EventDispatchers|BindEventtoOnTakeAnyDamage _returnvalue (delegate Custom|OnTakeAnyDamage)))
      (:Is%20Not%20Valid
        (Development|PrintString "no valid")))))

(fn GetHealth
  (return (Variables|Default|GetHealth)))

(fn SetHealth
  (params (NewHealth :type Float%20%28single-precision%29))
  (bind _output_get (LocalVariables|SetNextHealth (Math|Float|Clamp(Float) NewHealth 0.0 (Variables|Default|GetMaxHealth))))
  (bind _output_get_2 (LocalVariables|SetHealthDelta (- _output_get (Variables|Default|GetHealth))))
  (bind _output_get_3 (Variables|Default|SetHealth _output_get))
  (Default|CallOnHealthChanged _output_get_3 _output_get_2))

(fn HealUpdate
  (CallFunction|SetHealth (+ (Variables|Default|GetHealth) (Variables|Heal|GetHealModifier)))
  (bind _bishealthfull (CallFunction|IsHealthFull))
  (if _bishealthfull
    (Utilities|Time|ClearandInvalidateTimerbyHandle (Variables|Heal|GetHealTimer))))

(fn IsHealthFull
  (return (== (Variables|Default|GetHealth) (Variables|Default|GetMaxHealth))))

(fn IsDead
  (return (== (Variables|Default|GetHealth) 0.0)))

(fn GetHealthPercent
  (return (/ (Variables|Default|GetHealth) (Variables|Default|GetMaxHealth))))

(fn OnRepHealth)